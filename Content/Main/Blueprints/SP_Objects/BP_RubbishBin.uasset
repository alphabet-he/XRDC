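; BP_RubbishBin is a bin object that marks floating word actors for discarding.
; When its CollisionBox begins overlapping a BP_FloatingWordTemplate, it sets that word's ToDiscard flag, and clears it when the overlap ends.
; Both responses apply only while OnGround is true; the bin only sets the flag and performs no removal itself.
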(event `self.CollisionBox.OnComponentBeginOverlap`
  (params (OverlappedComponent :type "PrimitiveComponent Object Reference") (OtherActor :type "Actor Object Reference") (OtherComp :type "PrimitiveComponent Object Reference") (OtherBodyIndex :type Integer) (bFromSweep :type Boolean) (SweepResult :type "HitResult Structure (by ref)"))
  (if (`self.bOnGround`)
    (bind _asbp_floating_word_template (cast `/Game/Main/Blueprints/BP_FloatingWordTemplate` OtherActor))
    (set `/Game/Main/Blueprints/BP_FloatingWordTemplate.ToDiscard` true _asbp_floating_word_template)))

(event `self.CollisionBox.OnComponentEndOverlap`
  (params (OverlappedComponent :type "PrimitiveComponent Object Reference") (OtherActor :type "Actor Object Reference") (OtherComp :type "PrimitiveComponent Object Reference") (OtherBodyIndex :type Integer))
  (if (`self.bOnGround`)
    (bind _asbp_floating_word_template (cast `/Game/Main/Blueprints/BP_FloatingWordTemplate` OtherActor))
    (set `/Game/Main/Blueprints/BP_FloatingWordTemplate.ToDiscard` false _asbp_floating_word_template)))

(fn `UserConstructionScript`
  (`parent.UserConstructionScript`))