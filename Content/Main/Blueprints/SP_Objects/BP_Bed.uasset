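; BP_Bed is a grabbable bed object that controls whether the VR pawn is allowed to lie down and sleep on it.
; While the bed is on the ground, its collision box enables or disables lying down on overlapping pawns, with debug text.
; Grabbing the bed disables sleeping, and putting it down re-enables it for the player pawn.
; BeginPlay caches the sleep position's relative transform.
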(event `self.ReceiveBeginPlay`
  (`parent.ReceiveBeginPlay`)
  (set `self.SleepRelativeTrans` (`SceneComponent.GetRelativeTransform` (`self.SleepPosition`))))

(event `self.CollisionBox.OnComponentBeginOverlap`
  (params (OverlappedComponent :type "PrimitiveComponent Object Reference") (OtherActor :type "Actor Object Reference") (OtherComp :type "PrimitiveComponent Object Reference") (OtherBodyIndex :type Integer) (bFromSweep :type Boolean) (SweepResult :type "HitResult Structure (by ref)"))
  (if (`self.bOnGround`)
    (bind _asbp_my_vrpawn (cast `/Game/Main/Blueprints/Pawn/BP_MyVRPawn` OtherActor))
    (`/Game/Main/Blueprints/Pawn/BP_MyVRPawn.SetCanLayDown` _asbp_my_vrpawn true self)
    (`/Game/Main/Blueprints/Pawn/BP_MyVRPawn.SetDebugText` (`self.PlayerPawn`) "Can Sleep Now")))

(event `self.CollisionBox.OnComponentEndOverlap`
  (params (OverlappedComponent :type "PrimitiveComponent Object Reference") (OtherActor :type "Actor Object Reference") (OtherComp :type "PrimitiveComponent Object Reference") (OtherBodyIndex :type Integer))
  (if (`self.bOnGround`)
    (bind _asbp_my_vrpawn (cast `/Game/Main/Blueprints/Pawn/BP_MyVRPawn` OtherActor))
    (`/Game/Main/Blueprints/Pawn/BP_MyVRPawn.SetCanLayDown` _asbp_my_vrpawn false self)
    (`/Game/Main/Blueprints/Pawn/BP_MyVRPawn.SetDebugText` (`self.PlayerPawn`) "Cannot Sleep Now")))

(event `self.GrabComponent.OnGrabbed`
  (`/Game/Main/Blueprints/Pawn/BP_MyVRPawn.SetCanLayDown` (`self.PlayerPawn`) false null))

(fn `AfterPutToGround`
  (`/Game/Main/Blueprints/Pawn/BP_MyVRPawn.SetCanLayDown` (`self.PlayerPawn`) true self))

(fn `UserConstructionScript`
  (`parent.UserConstructionScript`))