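; BP_Tool_Fork is a grabbable VR fork that picks up interactable objects and removes them on contact with the player pawn.
; For category 0 interactions, it marks the object occupied, disables its GrabComponent, attaches its mesh and tracks it in an Attachment array.
; Dropping the fork clears occupancy, reactivates each grab component, calls TryRelease and empties the array.
; When its CollisionBox overlaps BP_MyVRPawn, all tracked objects are destroyed.
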(event `/Game/Main/Blueprints/BPI_Tool.InteractWithObject`
  (params (InteractingObject :type "/Game/Main/Blueprints/BP_ObjectTemplate Object Reference (by ref)") (Category :type "Integer (by ref)"))
  (switch `int` Category
    (:`0`
      (set `/Game/Main/Blueprints/BP_ObjectTemplate.bIsOccupied` true InteractingObject)
      (bind _asgrab_component (cast `/Game/VRTemplate/Blueprints/GrabComponent` (`FloatingWord.GrabComponent` InteractingObject)))
      (`/Game/VRTemplate/Blueprints/GrabComponent.TryRelease` _asgrab_component)
      (`ActorComponent.Deactivate` _asgrab_component)
      (`SceneComponent.K2_AttachToComponent` (`FloatingWord.Mesh` InteractingObject) (`self.Mesh`) "None" "KeepWorld" "KeepWorld" "KeepWorld" true)
      (`KismetArrayLibrary.Array_AddUnique` (`self.Attachment`) InteractingObject))))

(event `self.GrabComponent.OnDropped`
  (bind _attachment (`self.Attachment`))
  (if (> (`KismetArrayLibrary.Array_Length` _attachment) 0)
    (for _array_element _attachment
      (set `/Game/Main/Blueprints/BP_ObjectTemplate.bIsOccupied` false _array_element)
      (bind _asgrab_component (cast `/Game/VRTemplate/Blueprints/GrabComponent` (`FloatingWord.GrabComponent` _array_element)))
      (`ActorComponent.Activate` _asgrab_component false)
      (`/Game/VRTemplate/Blueprints/GrabComponent.TryRelease` _asgrab_component))
    (`KismetArrayLibrary.Array_Clear` (`self.Attachment`))))

(event `self.CollisionBox.OnComponentBeginOverlap`
  (params (OverlappedComponent :type "PrimitiveComponent Object Reference") (OtherActor :type "Actor Object Reference") (OtherComp :type "PrimitiveComponent Object Reference") (OtherBodyIndex :type Integer) (bFromSweep :type Boolean) (SweepResult :type "HitResult Structure (by ref)"))
  (cast `/Game/Main/Blueprints/BP_MyVRPawn` OtherActor)
  (if (> (`KismetArrayLibrary.Array_Length` (`self.Attachment`)) 0)
    (for _array_element (`self.Attachment`)
      (`self.K2_DestroyActor` _array_element))
    (`KismetArrayLibrary.Array_Clear` (`self.Attachment`))))

(fn `UserConstructionScript`
  (`parent.UserConstructionScript`))