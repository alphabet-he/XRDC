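; BP_FloatingWordTemplate is a floating word actor that rises from its start position and destroys itself unless grabbed.
; After a short delay on BeginPlay, FloatingTimeline lerps it up to UpperBoundary above StartPosition, adding a scaled sideways Deviation along DeviationDirection.
; When the timeline finishes, the actor waits briefly, then is destroyed.
; Grabbing it through GrabComponent stops the timeline, halting both the drift and the pending destruction.
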(event `self.ReceiveBeginPlay`
  (bind (_startposition_x _startposition_y _startposition_z) (`KismetMathLibrary.BreakVector` (`self.StartPosition`)))
  (`KismetSystemLibrary.Delay` 0.2)
  (bind _output_get (set `self.TargetPosition` (`KismetMathLibrary.MakeVector` _startposition_x _startposition_y (+ _startposition_z (`self.UpperBoundary`)))))
  (bind (_direction _z _deviation) (`Timeline|FloatingTimeline` :!via `PlayFromStart`)
    (:`Update`
      (`self.K2_SetActorLocation` (+ (`KismetMathLibrary.VLerp` (`self.StartPosition`) _output_get _z) (* _deviation (`self.DeviationDirection`) 30.0))))
    (:`Finished`
      (`KismetSystemLibrary.Delay` 2.0)
      (`self.K2_DestroyActor`))))

(event `self.GrabComponent.OnGrabbed`
  (`TimelineComponent.Stop` (`self.FloatingTimeline`)))

(fn `UserConstructionScript`)