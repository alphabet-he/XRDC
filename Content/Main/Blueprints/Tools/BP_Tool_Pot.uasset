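; BP_Tool_Pot is a cooking pot tool that turns attached ingredients into a grabbable dish.
; Interacting objects are released from grab and attached, starting pot tracing and a looping timer that waits for cooking.
; Cooking destroys ingredients, yielding nothing for only ice cream, otherwise a burned, bird or default carrot dish.
; The carrot check sits inside the bird check, so the combined carrot-bird dish is unreachable.
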(event `self.ReceiveBeginPlay`
  (`parent.ReceiveBeginPlay`))

(event `self.ReceiveTick`
  (params (DeltaSeconds :type "Float (single-precision)"))
  (`parent.ReceiveTick` DeltaSeconds))

(event `/Game/Main/Blueprints/BPI_Tool.InteractWithObject`
  (params (InteractingObject :type "/Game/Main/Blueprints/BP_ObjectTemplate Object Reference (by ref)") (Category :type "Integer (by ref)"))
  (bind _pot (`self.Pot`))
  (bind _asgrab_component (cast `/Game/VRTemplate/Blueprints/GrabComponent` (`FloatingWord.GrabComponent` InteractingObject)))
  (`/Game/VRTemplate/Blueprints/GrabComponent.TryRelease` _asgrab_component)
  (`ActorComponent.Deactivate` _asgrab_component)
  (`SceneComponent.K2_AttachToComponent` (`FloatingWord.Mesh` InteractingObject) (`self.Mesh`) "None" "KeepWorld" "KeepWorld" "KeepWorld" true)
  (set `/Game/Main/Blueprints/BP_ObjectTemplate.bIsAttached` true InteractingObject)
  (`KismetArrayLibrary.Array_AddUnique` (`self.Attachment`) InteractingObject)
  (`self.StartTracing` _pot)
  (bind _returnvalue (`KismetSystemLibrary.K2_SetTimerDelegate` (delegate `CheckTrace`) (`/Game/Main/Blueprints/Tools/BP_Tool_Pot.TraceDuration` _pot) true))
  (set `self.CheckTimer` _returnvalue))

(event `CheckTrace`
  (bind _returnvalue (`self.CheckTraceIsCooking` (`self.Pot`)))
  (`/Game/Main/Blueprints/Pawn/BP_MyVRPawn.SetDebugText` (`self.PlayerPawn`) (`KismetTextLibrary.Conv_BoolToText` _returnvalue))
  (if _returnvalue
    (`KismetSystemLibrary.K2_ClearAndInvalidateTimerHandle` (`self.CheckTimer`))
    (`self.Cook`)))

(event `Cook`
  (bind (_returnvalue_location _returnvalue_rotation) (`KismetMathLibrary.BreakTransform` (`SceneComponent.K2_GetComponentToWorld` (`self.CollisionBox`))))
  (bind _onlyicecream (`self.CheckOnlyIceCream`))
  (if _onlyicecream
    (`self.ClearAttachment`)
    (else
      (bind _returnvalue (`|SpawnActorFromClass` "/Game/Main/Blueprints/Others/BP_DishToGrab.BP_DishToGrab_C" (`KismetMathLibrary.MakeTransform` _returnvalue_location _returnvalue_rotation (0.1 0.1 0.1)) "AlwaysSpawn" "MultiplyWithRoot" null null))
      (bind _shouldburn (`self.CheckBurn`))
      (if _shouldburn
        (bind _staticmesh (`/Game/Main/Blueprints/Others/BP_DishToGrab.StaticMesh` _returnvalue))
        (`StaticMeshComponent.SetStaticMesh` _staticmesh (`self.BurnedDish`))
        (else
          (bind (_hasbird _hascarrot) (`self.CheckBirdCarrot`))
          (if (and _hasbird _hascarrot)
            (`StaticMeshComponent.SetStaticMesh` _staticmesh (`self.CarrotBirdDish`))
            (elif _hasbird
              (`StaticMeshComponent.SetStaticMesh` _staticmesh (`self.BirdDish`))
              (else
                (`StaticMeshComponent.SetStaticMesh` _staticmesh (`self.CarrotDish`)))))))
      (`self.ClearAttachment`)
      (`SceneComponent.K2_AttachToComponent` _staticmesh (`self.Mesh`) "None" "KeepWorld" "KeepWorld" "KeepWorld" true)
      (`ActorComponent.Activate` (`/Game/Main/Blueprints/Others/BP_DishToGrab.GrabComponent` _returnvalue) false)
      (`KismetArrayLibrary.Array_AddUnique` (`self.NonObjectAttachment`) _returnvalue))))

(fn `CheckBirdCarrot`
  (returns (HasBird :type Boolean) (HasCarrot :type Boolean))
  (locals (i_hasBird :type Boolean) (i_hasCarrot :type Boolean))
  (for _array_element (`self.Attachment`)
    (bind _objecttype (`/Game/Main/Blueprints/BP_ObjectTemplate.ObjectType` _array_element))
    (if (`|EnumEquality` _objecttype "BIRD")
      (set `local.i_hasBird` true)
      (if (`|EnumEquality` _objecttype "CARROT")
        (set `local.i_hasCarrot` true))))
  (return (`local.i_hasBird`) (`local.i_hasCarrot`)))

(fn `CheckBurn`
  (returns (ShouldBurn :type Boolean))
  (bind _output_objecttypes (break `ObjectTypeArr` (`|GetArrayItem` (`self.Categories`) 2)))
  (for _array_element (`self.Attachment`)
    (if (`KismetArrayLibrary.Array_Contains` _output_objecttypes (`/Game/Main/Blueprints/BP_ObjectTemplate.ObjectType` _array_element))
      (return true)))
  (return false))

(fn `CheckOnlyIceCream`
  (returns (OnlyIceCream :type Boolean))
  (bind _output_objecttypes (break `ObjectTypeArr` (`|GetArrayItem` (`self.Categories`))))
  (for _array_element (`self.Attachment`)
    (if (not (`KismetArrayLibrary.Array_Contains` _output_objecttypes (`/Game/Main/Blueprints/BP_ObjectTemplate.ObjectType` _array_element)))
      (return false)))
  (return true))

(fn `ClearAttachment`
  (bind _attachment (`self.Attachment`))
  (for _array_element _attachment
    (`self.K2_DestroyActor` _array_element))
  (`KismetArrayLibrary.Array_Clear` _attachment))

(fn `UserConstructionScript`
  (`parent.UserConstructionScript`))