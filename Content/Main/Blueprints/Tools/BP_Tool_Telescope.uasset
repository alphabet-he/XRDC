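; VR telescope tool that shows a magnified image of an attached object when the player looks into it.
; Interacting with an object releases its grab and attaches it to the mesh, one at a time, until it leaves CollisionBox.
; Pawn overlap with EyesCollision shows a MicroscopeWidget image looked up by object type, collapsed on exit.
; AfterPutToGround reattaches EyesCollision at the relative transform cached on BeginPlay.
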(event `self.ReceiveBeginPlay`
  (`parent.ReceiveBeginPlay`)
  (set `self.EyesCollisionRelativeTran` (`SceneComponent.GetRelativeTransform` (`self.EyesCollision`))))

(event `/Game/Main/Blueprints/BPI_Tool.InteractWithObject`
  (params (InteractingObject :type "/Game/Main/Blueprints/BP_ObjectTemplate Object Reference (by ref)") (Category :type "Integer (by ref)"))
  (bind _attachment (`self.Attachment`))
  (if (`KismetArrayLibrary.Array_IsEmpty` _attachment)
    (`|ExecutionSequence`
      (:`then_0`
        (`PrimitiveComponent.SetSimulatePhysics` (`FloatingWord.Mesh` InteractingObject) false))
      (:`then_1`
        (bind _asgrab_component (cast `/Game/VRTemplate/Blueprints/GrabComponent` (`FloatingWord.GrabComponent` InteractingObject)))
        (`/Game/VRTemplate/Blueprints/GrabComponent.TryRelease` _asgrab_component)
        (`ActorComponent.Deactivate` _asgrab_component)
        (`KismetSystemLibrary.Delay` 1.0)
        (`ActorComponent.Activate` _asgrab_component false))
      (:`then_2`
        (`SceneComponent.K2_AttachToComponent` (`FloatingWord.Mesh` InteractingObject) (`self.Mesh`) "None" "KeepWorld" "KeepWorld" "KeepWorld" true))
      (:`then_3`
        (`KismetArrayLibrary.Array_AddUnique` _attachment InteractingObject)))))

(event `self.CollisionBox.OnComponentEndOverlap`
  (params (OverlappedComponent :type "PrimitiveComponent Object Reference") (OtherActor :type "Actor Object Reference") (OtherComp :type "PrimitiveComponent Object Reference") (OtherBodyIndex :type Integer))
  (bind _attachment (`self.Attachment`))
  (bind _asbp_object_template (cast `/Game/Main/Blueprints/BP_ObjectTemplate` OtherActor))
  (if (`KismetArrayLibrary.Array_Contains` _attachment _asbp_object_template)
    (`KismetArrayLibrary.Array_Clear` _attachment)))

(event `self.EyesCollision.OnComponentBeginOverlap`
  (params (OverlappedComponent :type "PrimitiveComponent Object Reference") (OtherActor :type "Actor Object Reference") (OtherComp :type "PrimitiveComponent Object Reference") (OtherBodyIndex :type Integer) (bFromSweep :type Boolean) (SweepResult :type "HitResult Structure (by ref)"))
  (bind _microscopewidget (`self.MicroscopeWidget`))
  (bind _attachment (`self.Attachment`))
  (bind (_value _returnvalue) (`BlueprintMapLibrary.Map_Find` (`self.MicroscopeTexture`) (`/Game/Main/Blueprints/BP_ObjectTemplate.ObjectType` (`|GetArrayItem` _attachment))))
  (cast `/Game/Main/Blueprints/Pawn/BP_MyVRPawn` OtherActor)
  (if (`KismetArrayLibrary.Array_IsNotEmpty` _attachment)
    (if _returnvalue
      (`/Engine/EditorBlueprintResources/StandardMacros.IsValid` (`self.MicroscopeWidget`)
        (:`Is Valid`
          _)
        (:`Is Not Valid`
          (bind _returnvalue_2 (`|CreateWidget` "/Game/UI/WBP_MicroscopeWidget.WBP_MicroscopeWidget_C" (`GameplayStatics.GetPlayerController` 0)))
          (bind _output_get (set `self.MicroscopeWidget` _returnvalue_2))
          (`UserWidget.AddToViewport` _output_get 0)))
      (`/Game/UI/WBP_MicroscopeWidget.SetMicroscopeImage` _microscopewidget _value)
      (set `Widget.Visibility` "Visible" _microscopewidget))))

(event `self.EyesCollision.OnComponentEndOverlap`
  (params (OverlappedComponent :type "PrimitiveComponent Object Reference") (OtherActor :type "Actor Object Reference") (OtherComp :type "PrimitiveComponent Object Reference") (OtherBodyIndex :type Integer))
  (bind _microscopewidget (`self.MicroscopeWidget`))
  (cast `/Game/Main/Blueprints/Pawn/BP_MyVRPawn` OtherActor)
  (`/Engine/EditorBlueprintResources/StandardMacros.IsValid` _microscopewidget
    (:`Is Valid`
      (`Widget.SetVisibility` _microscopewidget "Collapsed"))))

(fn `AfterPutToGround`
  (bind _eyescollision (`self.EyesCollision`))
  (`parent.AfterPutToGround`)
  (`SceneComponent.K2_AttachToComponent` _eyescollision (`self.Mesh`) "None" "KeepWorld" "KeepWorld" "KeepWorld" true)
  (`SceneComponent.K2_SetRelativeTransform` _eyescollision (`self.EyesCollisionRelativeTran`) false false))

(fn `UserConstructionScript`
  (`parent.UserConstructionScript`))