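; VR fork tool that skewers objects, marks others, and feeds attached items to the player.
; InteractwithObject branches by category: categories 0 and 2 release the grab and attach to the fork mesh, while 1 traces through the collision box to place a canvas decal when the fork is empty.
; When CollisionBox overlaps the VR pawn, attached items are destroyed, with category 2 object types triggering a timed pink camera-fade illusion.
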(event `/Game/Main/Blueprints/BPI_Tool.InteractWithObject`
  (params (InteractingObject :type "/Game/Main/Blueprints/BP_ObjectTemplate Object Reference (by ref)") (Category :type "Integer (by ref)"))
  (bind _mesh (`FloatingWord.Mesh` InteractingObject))
  (bind _returnvalue (`SceneComponent.K2_GetComponentLocation` (`self.Mesh`)))
  (switch `int` Category
    (:`0`
      (bind _asgrab_component (cast `/Game/VRTemplate/Blueprints/GrabComponent` (`FloatingWord.GrabComponent` InteractingObject) :!label _label))
      (`/Game/VRTemplate/Blueprints/GrabComponent.TryRelease` _asgrab_component)
      (`ActorComponent.Deactivate` _asgrab_component)
      (set `/Game/Main/Blueprints/BP_ObjectTemplate.bIsAttached` true InteractingObject)
      (`SceneComponent.K2_AttachToComponent` _mesh (`self.Mesh`) "None" "KeepWorld" "KeepWorld" "KeepWorld" true)
      (`KismetArrayLibrary.Array_AddUnique` (`self.Attachment`) InteractingObject))
    (:`1`
      (if (not (> (`KismetArrayLibrary.Array_Length` (`self.Attachment`)) 0))
        (bind _outhit (`KismetSystemLibrary.LineTraceSingle` _returnvalue (+ _returnvalue (* (- (`SceneComponent.K2_GetComponentLocation` (`self.CollisionBox`)) _returnvalue) 100.0)) "TraceTypeQuery1"))
        (if (== (`.HitActor` (`GameplayStatics.BreakHitResult` _outhit)) InteractingObject)
          (`GameplayStatics.SpawnDecalAttached` "/Game/Asset/Material_Inst/MI_CanvasDecal.MI_CanvasDecal" (2.0 2.0 2.0) _mesh "None" (`.Location` (`GameplayStatics.BreakHitResult` _outhit)) (struct) "KeepWorldPosition"))))
    (:`2`
      (goto _label))))

(event `self.CollisionBox.OnComponentBeginOverlap`
  (params (OverlappedComponent :type "PrimitiveComponent Object Reference") (OtherActor :type "Actor Object Reference") (OtherComp :type "PrimitiveComponent Object Reference") (OtherBodyIndex :type Integer) (bFromSweep :type Boolean) (SweepResult :type "HitResult Structure (by ref)"))
  (bind _output_objecttypes (break `ObjectTypeArr` (`|GetArrayItem` (`self.Categories`) 2)))
  (cast `/Game/Main/Blueprints/Pawn/BP_MyVRPawn` OtherActor)
  (if (> (`KismetArrayLibrary.Array_Length` (`self.Attachment`)) 0)
    (for _array_element (`self.Attachment`)
      (if (`KismetArrayLibrary.Array_Contains` _output_objecttypes (`/Game/Main/Blueprints/BP_ObjectTemplate.ObjectType` _array_element))
        (`self.StartIllusion`))
      (`self.K2_DestroyActor` _array_element))
    (`KismetArrayLibrary.Array_Clear` (`self.Attachment`))))

(event `StartIllusion`
  (bind _returnvalue (`GameplayStatics.GetPlayerCameraManager` 0))
  (`PlayerCameraManager.StartCameraFade` _returnvalue 0.0 0.7 1.5 (struct :`R` 1.0 :`G` 0.101729 :`B` 0.994442 :`A` 1.0) false true)
  (`KismetSystemLibrary.Delay` 1.5)
  (`PlayerCameraManager.StartCameraFade` _returnvalue 0.7 0.0 1.5 (struct :`R` 1.0 :`G` 0.101961 :`B` 0.996078 :`A` 1.0) false true)
  (`KismetSystemLibrary.Delay` 1.5)
  (`PlayerCameraManager.StopCameraFade` _returnvalue))

(fn `UserConstructionScript`
  (`parent.UserConstructionScript`))