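; Watering can tool that waters, grows or knocks down the objects it interacts with.
; Interaction only fires while the mesh origin sits more than a set height above the collision box, apparently serving as a pouring check.
; The passed category picks the response: call PouredWater, call Grow, or cast to a bird and make it fall to the ground.
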(event `self.ReceiveBeginPlay`
  (`parent.ReceiveBeginPlay`))

(event `/Game/Main/Blueprints/BPI_Tool.InteractWithObject`
  (params (InteractingObject :type "/Game/Main/Blueprints/BP_ObjectTemplate Object Reference (by ref)") (Category :type "Integer (by ref)"))
  (bind (_returnvalue_x _returnvalue_y _returnvalue_z) (`KismetMathLibrary.BreakVector` (`SceneComponent.K2_GetComponentLocation` (`self.CollisionBox`))))
  (bind (_returnvalue_x_2 _returnvalue_y_2 _returnvalue_z_2) (`KismetMathLibrary.BreakVector` (`SceneComponent.K2_GetComponentLocation` (`self.Mesh`))))
  (if (> (- _returnvalue_z_2 _returnvalue_z) 55.0)
    (switch `int` Category
      (:`0`
        (`/Game/Main/Blueprints/BP_ObjectTemplate.PouredWater` InteractingObject))
      (:`1`
        (`/Game/Main/Blueprints/BP_ObjectTemplate.Grow` InteractingObject))
      (:`2`
        (bind _asbp_object_bird (cast `/Game/Main/Blueprints/Objects/BP_Object_Bird` InteractingObject))
        (`/Game/Main/Blueprints/Objects/BP_Object_Bird.FallToGround` _asbp_object_bird)))))

(event `self.ReceiveTick`
  (params (DeltaSeconds :type "Float (single-precision)")))

(fn `UserConstructionScript`
  (`parent.UserConstructionScript`))