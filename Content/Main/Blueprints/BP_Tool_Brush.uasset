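; BP_Tool_Brush is a grabbable brush tool that paints by leaving a trail of short-lived decals.
; An InteractwithObject event with the first category turns drawing on.
; While drawing, Tick spawns a small, fixed-rotation BaseMaterial decal at the CollisionBox location every frame.
; Drawing stops when the box ends overlap with a BP_ObjectTemplate actor or the GrabComponent reports a drop.
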(event `self.ReceiveTick`
  (params (DeltaSeconds :type "Float (single-precision)"))
  (`parent.ReceiveTick` DeltaSeconds)
  (if (`self.bIsDrawing`)
    (`GameplayStatics.SpawnDecalAtLocation` "/Game/FPWeapon/Materials/BaseMaterial.BaseMaterial" (0.1 0.1 0.1) (`SceneComponent.K2_GetComponentLocation` (`self.CollisionBox`)) (struct) 2.0)))

(event `/Game/Main/Blueprints/BPI_Tool.InteractWithObject`
  (params (InteractingObject :type "/Game/Main/Blueprints/BP_ObjectTemplate Object Reference (by ref)") (Category :type "Integer (by ref)"))
  (switch `int` Category
    (:`0`
      (set `self.bIsDrawing` true))))

(event `self.CollisionBox.OnComponentEndOverlap`
  (params (OverlappedComponent :type "PrimitiveComponent Object Reference") (OtherActor :type "Actor Object Reference") (OtherComp :type "PrimitiveComponent Object Reference") (OtherBodyIndex :type Integer))
  (cast `/Game/Main/Blueprints/BP_ObjectTemplate` OtherActor)
  (set `self.bIsDrawing` false))

(event `self.GrabComponent.OnDropped`
  (set `self.bIsDrawing` false))

(fn `UserConstructionScript`
  (`parent.UserConstructionScript`))