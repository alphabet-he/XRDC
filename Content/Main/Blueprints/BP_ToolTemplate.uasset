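; Base Blueprint for grabbable tools that interact with held objects touching their collision box.
; An overlap counts when the tool is held or, for ground-placeable tools, resting on the ground.
; It matches the object's type to a category, marks it used and passes both to InteractWithObject.
; First grab notifies BP_ToolTelevision; once grabbed, Tick keeps the box's location following the mesh.
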(event `self.ReceiveBeginPlay`
  (`parent.ReceiveBeginPlay`)
  (set `self.bIsTool` true))

(event `self.CollisionBox.OnComponentBeginOverlap`
  (params (OverlappedComponent :type "PrimitiveComponent Object Reference") (OtherActor :type "Actor Object Reference") (OtherComp :type "PrimitiveComponent Object Reference") (OtherBodyIndex :type Integer) (bFromSweep :type Boolean) (SweepResult :type "HitResult Structure (by ref)"))
  (if (`self.bCanPutToGround`)
    (if (`self.bOnGround`)
      (bind _asbp_object_template (cast `/Game/Main/Blueprints/BP_ObjectTemplate` OtherActor :!label _label))
      (bind _asgrab_component (cast `/Game/VRTemplate/Blueprints/GrabComponent` (`FloatingWord.GrabComponent` _asbp_object_template)))
      (if (`/Game/VRTemplate/Blueprints/GrabComponent.bIsHeld` _asgrab_component)
        (bind _category (`self.GetCategory` (`/Game/Main/Blueprints/BP_ObjectTemplate.ObjectType` _asbp_object_template)))
        (if (>= _category 0)
          (set `FloatingWord.bUsed` true _asbp_object_template)
          (`/Game/Main/Blueprints/BPI_Tool.InteractWithObject` _asbp_object_template _category))))
    (else
      (bind _asgrab_component_2 (cast `/Game/VRTemplate/Blueprints/GrabComponent` (`self.GrabComponent`)))
      (if (`/Game/VRTemplate/Blueprints/GrabComponent.bIsHeld` _asgrab_component_2)
        (goto _label)))))

(event `self.GrabComponent.OnGrabbed`
  (set `self.bUpdateCollisionTransform` true)
  (if (not (`self.bUsed`))
    (bind _returnvalue (`GameplayStatics.GetActorOfClass` "/Game/Main/Blueprints/Others/BP_ToolTelevision.BP_ToolTelevision_C"))
    (`ToolTelevision.ToolGrabbed` _returnvalue)
    (set `self.bUsed` true)))

(event `self.ReceiveTick`
  (params (DeltaSeconds :type "Float (single-precision)"))
  (bind _collisionrelativetrans_location (`KismetMathLibrary.BreakTransform` (`self.CollisionRelativeTrans`)))
  (if (`self.bUpdateCollisionTransform`)
    (`SceneComponent.K2_SetWorldLocation` (`self.CollisionBox`) (`KismetMathLibrary.TransformLocation` (`SceneComponent.K2_GetComponentToWorld` (`self.Mesh`)) _collisionrelativetrans_location) false true)))

(fn `GetCategory`
  (params (ObjectType :type "EObjects Enum" :default "PANCAKE"))
  (returns (Category :type Integer))
  (bind _categories (`self.Categories`))
  (for _index (range (`KismetArrayLibrary.Array_Length` _categories))
    (bind _output_objecttypes (break `ObjectTypeArr` (`|GetArrayItem` _categories _index)))
    (if (`KismetArrayLibrary.Array_Contains` _output_objecttypes ObjectType)
      (return _index)))
  (return -1))

(fn `UserConstructionScript`
  (`parent.UserConstructionScript`))