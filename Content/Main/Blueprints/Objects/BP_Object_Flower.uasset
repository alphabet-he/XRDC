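; BP_Object_Flower is a grabbable flower object that can dance.
; The Dance event sets a dancing flag and plays a timeline from the start, whose Height track drives the mesh's relative Z position while X and Y stay unchanged.
; Grabbing it through GrabComponent clears the flag and stops the timeline, without resetting the mesh height.
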(event `/Game/Main/Blueprints/BPI_Object.Dance`
  (bind _mesh (`self.Mesh`))
  (bind (_relativelocation_x _relativelocation_y) (`KismetMathLibrary.BreakVector` (`SceneComponent.RelativeLocation` _mesh)))
  (set `self.isDancing` true)
  (bind (_direction _height) (`Timeline|DanceTimeline` :!via `PlayFromStart`)
    (:`Update`
      (`SceneComponent.K2_SetRelativeLocation` _mesh (`KismetMathLibrary.MakeVector` _relativelocation_x _relativelocation_y (* _height 60.0)) false false))))

(event `self.GrabComponent.OnGrabbed`
  (if (`self.isDancing`)
    (set `self.isDancing` false)
    (`TimelineComponent.Stop` (`self.DanceTimeline`))))

(fn `UserConstructionScript`
  (`parent.UserConstructionScript`))