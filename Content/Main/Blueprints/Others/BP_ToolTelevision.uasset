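; VR television with power, next and confirm buttons, apparently for choosing the player's tool.
; An interaction area toggles hand-collision updates on the VR pawn, and buttons respond only to overlaps from BP_CollisionCheckingHelper actors.
; A successful confirm sweeps all BP_ToolTemplate actors not matching the ToolList class at PrevGrabbedToolInd.
; These lose their attachments and grab, then used ones are rescaled and float away while unused ones are destroyed.
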(event `self.InteractionArea.OnComponentBeginOverlap`
  (params (OverlappedComponent :type "PrimitiveComponent Object Reference") (OtherActor :type "Actor Object Reference") (OtherComp :type "PrimitiveComponent Object Reference") (OtherBodyIndex :type Integer) (bFromSweep :type Boolean) (SweepResult :type "HitResult Structure (by ref)"))
  (bind _asbp_my_vrpawn (cast `/Game/Main/Blueprints/Pawn/BP_MyVRPawn` OtherActor))
  (set `/Game/Main/Blueprints/Pawn/BP_MyVRPawn.NeedUpdateHandCollision` true _asbp_my_vrpawn)
  (`/Game/Main/Blueprints/Pawn/BP_MyVRPawn.SetDebugText` _asbp_my_vrpawn "In Tele Interaction"))

(event `self.InteractionArea.OnComponentEndOverlap`
  (params (OverlappedComponent :type "PrimitiveComponent Object Reference") (OtherActor :type "Actor Object Reference") (OtherComp :type "PrimitiveComponent Object Reference") (OtherBodyIndex :type Integer))
  (bind _asbp_my_vrpawn (cast `/Game/Main/Blueprints/Pawn/BP_MyVRPawn` OtherActor))
  (set `/Game/Main/Blueprints/Pawn/BP_MyVRPawn.NeedUpdateHandCollision` false _asbp_my_vrpawn)
  (`/Game/Main/Blueprints/Pawn/BP_MyVRPawn.SetDebugText` _asbp_my_vrpawn "Out tele interaction"))

(event `self.PowerButtonCollision.OnComponentBeginOverlap`
  (params (OverlappedComponent :type "PrimitiveComponent Object Reference") (OtherActor :type "Actor Object Reference") (OtherComp :type "PrimitiveComponent Object Reference") (OtherBodyIndex :type Integer) (bFromSweep :type Boolean) (SweepResult :type "HitResult Structure (by ref)"))
  (cast `/Game/Main/Blueprints/Pawn/BP_CollisionCheckingHelper` OtherActor)
  (`self.HitPowerButton`))

(event `self.NextButtonCollision.OnComponentBeginOverlap`
  (params (OverlappedComponent :type "PrimitiveComponent Object Reference") (OtherActor :type "Actor Object Reference") (OtherComp :type "PrimitiveComponent Object Reference") (OtherBodyIndex :type Integer) (bFromSweep :type Boolean) (SweepResult :type "HitResult Structure (by ref)"))
  (cast `/Game/Main/Blueprints/Pawn/BP_CollisionCheckingHelper` OtherActor)
  (`self.HitNextButton`))

(event `self.ConfirmButtonCollision.OnComponentBeginOverlap`
  (params (OverlappedComponent :type "PrimitiveComponent Object Reference") (OtherActor :type "Actor Object Reference") (OtherComp :type "PrimitiveComponent Object Reference") (OtherBodyIndex :type Integer) (bFromSweep :type Boolean) (SweepResult :type "HitResult Structure (by ref)"))
  (cast `/Game/Main/Blueprints/Pawn/BP_CollisionCheckingHelper` OtherActor)
  (bind _returnvalue (`self.HitConfirmButton`))
  (if _returnvalue
    (bind _outactors (`GameplayStatics.GetAllActorsOfClass` "/Game/Main/Blueprints/BP_ToolTemplate.BP_ToolTemplate_C"))
    (for _array_element _outactors
      (if (not (== (`|GetArrayItem` (`self.ToolList`) (`KismetMathLibrary.Conv_ByteToInt` (`self.PrevGrabbedToolInd`))) (`GameplayStatics.GetObjectClass` _array_element)))
        (`|ExecutionSequence`
          (:`then_0`
            (bind _attachment (`/Game/Main/Blueprints/BP_ToolTemplate.Attachment` _array_element))
            (for _array_element_2 _attachment
              (`self.K2_DestroyActor` _array_element_2))
            (`KismetArrayLibrary.Array_Clear` _attachment)
            (bind _nonobjectattachment (`/Game/Main/Blueprints/BP_ToolTemplate.NonObjectAttachment` _array_element))
            (for _array_element_3 _nonobjectattachment
              (`self.K2_DestroyActor` _array_element_3))
            (`KismetArrayLibrary.Array_Clear` _nonobjectattachment))
          (:`then_1`
            (bind _asgrab_component (cast `/Game/VRTemplate/Blueprints/GrabComponent` (`FloatingWord.GrabComponent` _array_element)))
            (`/Game/VRTemplate/Blueprints/GrabComponent.TryRelease` _asgrab_component)
            (`ActorComponent.Deactivate` _asgrab_component))
          (:`then_2`
            (if (`FloatingWord.bUsed` _array_element)
              (bind _mesh (`FloatingWord.Mesh` _array_element))
              (`PrimitiveComponent.SetSimulatePhysics` _mesh false)
              (`SceneComponent.K2_AttachToComponent` _mesh (`Actor.RootComponent` _array_element) "None" "KeepWorld" "KeepWorld" "KeepWorld" true)
              (bind _inhandscale (`FloatingWord.InHandScale` _array_element))
              (`SceneComponent.SetWorldScale3D` _mesh (`KismetMathLibrary.MakeVector` _inhandscale _inhandscale _inhandscale))
              (`/Game/Main/Blueprints/BP_FloatingWordTemplate.FloatAway` _array_element)
              (else
                (`self.K2_DestroyActor` _array_element)))))))))

(fn `UserConstructionScript`)