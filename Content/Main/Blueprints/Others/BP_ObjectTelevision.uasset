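; VR television prop with a power button the player triggers by physical overlap.
; An InteractionArea sets NeedUpdateHandCollision on BP_MyVRPawn while it is inside, including a check at BeginPlay for a pawn already overlapping.
; When a BP_CollisionCheckingHelper enters PowerButtonCollision, HitPowerButton is called; its logic is not defined in these graphs.
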(event `self.ReceiveBeginPlay`
  (bind _overlappingactors (`PrimitiveComponent.GetOverlappingActors` (`self.InteractionArea`) "/Game/Main/Blueprints/Pawn/BP_MyVRPawn.BP_MyVRPawn_C"))
  (if (`KismetArrayLibrary.Array_IsNotEmpty` _overlappingactors)
    (bind _asbp_my_vrpawn (cast `/Game/Main/Blueprints/Pawn/BP_MyVRPawn` (`|GetArrayItem` _overlappingactors)))
    (set `/Game/Main/Blueprints/Pawn/BP_MyVRPawn.NeedUpdateHandCollision` true _asbp_my_vrpawn)))

(event `self.InteractionArea.OnComponentBeginOverlap`
  (params (OverlappedComponent :type "PrimitiveComponent Object Reference") (OtherActor :type "Actor Object Reference") (OtherComp :type "PrimitiveComponent Object Reference") (OtherBodyIndex :type Integer) (bFromSweep :type Boolean) (SweepResult :type "HitResult Structure (by ref)"))
  (bind _asbp_my_vrpawn (cast `/Game/Main/Blueprints/Pawn/BP_MyVRPawn` OtherActor))
  (set `/Game/Main/Blueprints/Pawn/BP_MyVRPawn.NeedUpdateHandCollision` true _asbp_my_vrpawn))

(event `self.InteractionArea.OnComponentEndOverlap`
  (params (OverlappedComponent :type "PrimitiveComponent Object Reference") (OtherActor :type "Actor Object Reference") (OtherComp :type "PrimitiveComponent Object Reference") (OtherBodyIndex :type Integer))
  (bind _asbp_my_vrpawn (cast `/Game/Main/Blueprints/Pawn/BP_MyVRPawn` OtherActor))
  (set `/Game/Main/Blueprints/Pawn/BP_MyVRPawn.NeedUpdateHandCollision` false _asbp_my_vrpawn))

(event `self.PowerButtonCollision.OnComponentBeginOverlap`
  (params (OverlappedComponent :type "PrimitiveComponent Object Reference") (OtherActor :type "Actor Object Reference") (OtherComp :type "PrimitiveComponent Object Reference") (OtherBodyIndex :type Integer) (bFromSweep :type Boolean) (SweepResult :type "HitResult Structure (by ref)"))
  (cast `/Game/Main/Blueprints/Pawn/BP_CollisionCheckingHelper` OtherActor)
  (`self.HitPowerButton`))

(fn `UserConstructionScript`)